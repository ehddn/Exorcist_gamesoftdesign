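; BP_TestCharacter is a test character Blueprint that drives an encounter counter leading to a level change.
; While the encounter flag is set, Tick adds a fixed amount per frame, independent of delta time, and prints the value.
; When the counter reaches its threshold, Tick opens NewMap by name.
; SetencountTrue raises the flag, and SetencountFalse clears it and resets the counter.
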(event EventBeginPlay)

(event Collision|EventActorBeginOverlap
  (params (OtherActor :type Actor%20Object%20Reference)))

(event EventTick
  (params (DeltaSeconds :type Float%20%28single-precision%29))
  (Variables|Default|SetTick_var DeltaSeconds)
  (Utilities|FlowControl|Sequence
    (:then_0
      (if (Math|Boolean|Equal(Boolean) true (Variables|Default|GetIsEncount_2))
        (bind _output_get (Variables|Default|Setencount (+ (Variables|Default|Getencount) 0.5)))
        (Development|PrintString (Utilities|String|ToString(Float) _output_get))
        (else
          (Variables|Default|SetIsEncount_2 false))))
    (:then_1
      (if (>= (Variables|Default|Getencount) 1e+02)
        (Game|OpenLevel(byName) "NewMap")))))

(fn ConstructionScript)

(fn SetencountTrue
  (Variables|Default|SetIsEncount_2 true))

(fn SetencountFalse
  (Variables|Default|SetIsEncount_2 false)
  (Variables|Default|Setencount 0.0))