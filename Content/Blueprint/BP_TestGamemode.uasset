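; Test game mode that sets up the shop UI and offers a keyboard shortcut to open and close it.
; BeginPlay creates the shop icon widget and adds it to the viewport, creates but only stores the main shop widget, then enables input from player controller 0.
; P calls open or close on the icon widget based on IsShowShop, whose setters here are unconnected.
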(event EventBeginPlay
  ;[1 1 1] 상점아이콘 및 상점 UI 변수화 승격
  (Utilities|FlowControl|Sequence
    (:then_0
      (bind _returnvalue (UserInterface|CreateWidget "/Game/UI/UI_Shop_Icon.UI_Shop_Icon_C"))
      (Variables|Default|SetUI_shopIcon _returnvalue)
      (UserInterface|Viewport|AddtoViewport (Variables|Default|GetUI_shopIcon) 0))
    (:then_1
      (bind _returnvalue_2 (UserInterface|CreateWidget "/Game/UI/UI_ShopMain.UI_ShopMain_C"))
      (Variables|Default|SetUI_ShopMain _returnvalue_2))
    (:then_2
      ;[1 1 1] 게임모드에서 입력받기위해 플레이어컨트롤러를 가져와 항상 입력이 가능한 상태로 만듬
      (Input|EnableInput (Game|GetPlayerController 0)))))

(event EventTick
  (params (DeltaSeconds :type Float%20%28single-precision%29)))

(event Input|KeyboardEvents|P
  (params (Key :type Key%20Structure :default "None"))
  (bind _ui_shopicon (Variables|Default|GetUI_shopIcon))
  ;[1 1 1] p누를시 상점창 오픈(토글)(상의해본후 필요없는기능일시 삭제)
  (:Pressed
    (if (Math|Boolean|Equal(Boolean) false (Variables|Default|GetIsShow_Shop))
      (Default|OpenShop _ui_shopicon)
      (else
        (Default|상점닫기 _ui_shopicon)))))

(fn ConstructionScript)